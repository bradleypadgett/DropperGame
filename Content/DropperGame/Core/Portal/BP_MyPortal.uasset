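; Portal actor in DropperGame that displays the view captured by a linked portal on its plane.
; The construction script gives its SceneCaptureComponent2D a new square canvas render target, then feeds the PortalLink's capture target into a dynamic material on the plane.
; With TransitionPortal set, a linked portal shows a green galaxy sky material instead.
; The event graph is empty, so this Blueprint's graphs handle only visuals, with no teleport logic.
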(fn `UserConstructionScript`
  (bind _returnvalue (`CanvasRenderTarget2D.CreateCanvasRenderTarget2D` "/Script/Engine.CanvasRenderTarget2D"))
  (set `SceneCaptureComponent2D.TextureTarget` _returnvalue (`self.SceneCaptureComponent2D`))
  (`self.Portal Link`
    (:`then`
      (if (`self.TransitionPortal`)
        (`PrimitiveComponent.CreateDynamicMaterialInstance` (`self.Plane`) 0 "/Game/DropperGame/Core/Portal/MI_Sky_GreenGalaxy.MI_Sky_GreenGalaxy" "None")
        (else
          (bind _returnvalue_2 (`PrimitiveComponent.CreateDynamicMaterialInstance` (`self.Plane`) 0 "/Game/DropperGame/Core/Portal/M_PortalRenderTarget.M_PortalRenderTarget" "None"))
          (`MaterialInstanceDynamic.SetTextureParameterValue` _returnvalue_2 "Texture" (`SceneCaptureComponent2D.TextureTarget` (`/Game/DropperGame/Core/Portal/BP_MyPortal.SceneCaptureComponent2D` (`self.Portal Link`)))))))
    (:`else`)))